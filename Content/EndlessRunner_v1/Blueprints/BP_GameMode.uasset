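; Game mode for an endless runner that procedurally builds the track and shows the HUD.
; On BeginPlay it adds WB_HUD to the viewport and spawns an initial run of floor tiles.
; AddFloorTile spawns a random straight BP_Floor class, switching to AddFloorTurn for a random turn piece once enough straights accumulate.
; Each piece's attach transform becomes the next spawn point, chaining the tiles.
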(event `self.ReceiveBeginPlay`
  (bind _returnvalue (`|CreateWidget` "/Game/EndlessRunner_v1/Blueprints/WB_HUD.WB_HUD_C"))
  (`UserWidget.AddToViewport` _returnvalue 0)
  (for _ (range 10)
    (`self.AddFloorTile`)))

(fn `AddFloorTile`
  (bind _floorspawn (`self.FloorSpawn`))
  (if (> (`self.Straights`) 7)
    (`self.AddFloorTurn`)
    (else
      (bind _returnvalue (`|SpawnActorFromClass` (`|GetArrayItem` _floorspawn (`KismetMathLibrary.RandomIntegerInRange` 0 (`KismetArrayLibrary.Array_LastIndex` _floorspawn))) (`self.NextSpawnPoint`) "Undefined" "OverrideRootScale" null null))
      (bind _asbp_floor (cast `/Game/EndlessRunner_v1/Blueprints/BP_Floor` _returnvalue))
      (bind _attachtransform (`/Game/EndlessRunner_v1/Blueprints/BP_Floor.GetAttachTransform` _asbp_floor))
      (set `self.NextSpawnPoint` _attachtransform)
      (set `self.Straights` (+ (`self.Straights`) 1)))))

(fn `AddFloorTurn`
  (bind _turnfloorspawn (`self.TurnFloorSpawn`))
  (bind _returnvalue (`|SpawnActorFromClass` (`|GetArrayItem` _turnfloorspawn (`KismetMathLibrary.RandomIntegerInRange` 0 (`KismetArrayLibrary.Array_LastIndex` _turnfloorspawn))) (`self.NextSpawnPoint`) "Undefined" "OverrideRootScale" null null))
  (bind _asbp_floor (cast `/Game/EndlessRunner_v1/Blueprints/BP_Floor` _returnvalue))
  (bind _attachtransform (`/Game/EndlessRunner_v1/Blueprints/BP_Floor.GetAttachTransform` _asbp_floor))
  (set `self.NextSpawnPoint` _attachtransform)
  (set `self.Straights` 0))

(fn `UserConstructionScript`)
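; BP_Floor is a floor tile for the endless runner that randomly fills itself with either an obstacle or coins.
; The construction script places one obstacle at a random left, center or right spawn point, or scatters coins inside a box.
; Overlapping the end trigger makes BP_GameMode add another tile, then this one destroys itself after a short delay.
; Side walls kill the character only on head-on hits, detected by comparing hit normal with forward vector.
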(event `self.EndTrigger.OnComponentBeginOverlap`
  (params (OverlappedComponent :type "PrimitiveComponent Object Reference") (OtherActor :type "Actor Object Reference") (OtherComp :type "PrimitiveComponent Object Reference") (OtherBodyIndex :type Integer) (bFromSweep :type Boolean) (SweepResult :type "HitResult Structure (by ref)"))
  (cast `/Game/EndlessRunner_v1/Blueprints/BP_Character` OtherActor)
  (bind _asbp_game_mode (cast `/Game/EndlessRunner_v1/Blueprints/BP_GameMode` (`GameplayStatics.GetGameMode`)))
  (`/Game/EndlessRunner_v1/Blueprints/BP_GameMode.AddFloorTile` _asbp_game_mode)
  (`KismetSystemLibrary.Delay` 2.0)
  (`self.K2_DestroyActor`))

(event `self.Wall_R.OnComponentHit`
  (params (HitComponent :type "PrimitiveComponent Object Reference") (OtherActor :type "Actor Object Reference") (OtherComp :type "PrimitiveComponent Object Reference") (NormalImpulse :type "Vector Structure") (Hit :type "HitResult Structure (by ref)"))
  (bind _asbp_character (cast `/Game/EndlessRunner_v1/Blueprints/BP_Character` OtherActor))
  (if (`KismetMathLibrary.NearlyEqual_FloatFloat` (`KismetMathLibrary.Dot_VectorVector` Hit_Normal (`self.GetActorForwardVector` _asbp_character)) -1.0 0.01)
    (`/Game/EndlessRunner_v1/Blueprints/BP_Character.Death` _asbp_character)))

(event `self.Wall_L.OnComponentHit`
  (params (HitComponent :type "PrimitiveComponent Object Reference") (OtherActor :type "Actor Object Reference") (OtherComp :type "PrimitiveComponent Object Reference") (NormalImpulse :type "Vector Structure") (Hit :type "HitResult Structure (by ref)"))
  (bind _asbp_character (cast `/Game/EndlessRunner_v1/Blueprints/BP_Character` OtherActor))
  (if (`KismetMathLibrary.NearlyEqual_FloatFloat` (`KismetMathLibrary.Dot_VectorVector` Hit_Normal (`self.GetActorForwardVector` _asbp_character)) -1.0 0.01)
    (`/Game/EndlessRunner_v1/Blueprints/BP_Character.Death` _asbp_character)))

(fn `GetAttachTransform`
  (returns (AttachTransform :type "Transform Structure"))
  (return (`SceneComponent.K2_GetComponentToWorld` (`self.AttachPoint`))))

(fn `SetSpawnPoints`
  (set `self.SpawnPoints` (`|MakeArray` (`SceneComponent.GetRelativeTransform` (`self.SpawnPointR`)) (`SceneComponent.GetRelativeTransform` (`self.SpawnPointC`)) (`SceneComponent.GetRelativeTransform` (`self.SpawnPointL`)))))

(fn `SpawnCoin`
  (bind _spawncollectable (`self.SpawnCollectable`))
  (for _ (range 6)
    (`AddComponent|NODE_AddChildActorComponent-1` :`RelativeTransform` (`KismetMathLibrary.Conv_VectorToTransform` (`KismetMathLibrary.RandomPointInBoundingBox` (`SceneComponent.RelativeLocation` _spawncollectable) (`BoxComponent.BoxExtent` _spawncollectable))))))

(fn `SpawnObstackle`
  (bind _spawnpoints (`self.SpawnPoints`))
  (`AddComponent|NODE_AddChildActorComponent-0` :`RelativeTransform` (`|GetArrayItem` _spawnpoints (`KismetMathLibrary.RandomIntegerInRange` 0 (`KismetArrayLibrary.Array_LastIndex` _spawnpoints)))))

(fn `UserConstructionScript`
  (`self.SetSpawnPoints`)
  (switch `int` (`KismetMathLibrary.RandomIntegerInRange` 0 1)
    (:`Default`
      (`self.SpawnObstackle` :!label _label))
    (:`0`
      (goto _label))
    (:`1`
      (`self.SpawnCoin`))))